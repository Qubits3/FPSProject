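; Master AI enemy character that holds a gun, runs the BT_AIEnemy behavior tree and shows its health on a WP_HealthBar widget.
; Projectile hits subtract fixed damage, refresh the bar and call Die.
; At exactly zero health, Die flags the blackboard, ragdolls the body, disables capsule collision, detaches the gun, clears the widget and destroys the actor after a delay.
; The construction script snaps the gun to the body's GripPoint socket.
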(event `self.ReceiveBeginPlay`
  (`self.SetHealthToWidget`)
  (`AIController.RunBehaviorTree` (`AIBlueprintHelperLibrary.GetAIController` self) "/Game/Characters/AIEnemy/BT_AIEnemy.BT_AIEnemy"))

(event `/Game/Blueprints/BPI_Damage.ApplyProjectileDamage`
  (bind _health (`self.Health`))
  (if (> _health 0.0)
    (set `self.Health` (- _health 10.0))
    (`self.SetHealthToWidget`)
    (`self.Die`)))

(fn `UserConstructionScript`
  (`SceneComponent.K2_AttachToComponent` (`self.Gun`) (`self.Body`) "GripPoint" "SnapToTarget" "KeepRelative" "SnapToTarget" true))