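; Base AI enemy character that runs a behavior tree, carries a socketed gun and shows a health bar.
; Perception writes player visibility and last stimulus location to the blackboard.
; Damage lowers health, updates the bar and flashes the HUD hit crosshair.
; At zero health it flags the blackboard, awards score, ragdolls, hides the gun, clears the widget, calls the overridable OnDie and destroys itself after a delay.
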(event `SetBehaviorTree`
  (params (BTAsset :type "BehaviorTree Object Reference"))
  ;[1 0 0] Every child must call this event on BeginPlay
  (`AIController.RunBehaviorTree` (`AIBlueprintHelperLibrary.GetAIController` self) BTAsset))

(event `self.ReceiveBeginPlay`
  (`self.SetHealthToWidget`)
  (`self.SetBehaviorTree` "/Game/AIEnemies/Master/BT_AIEnemyMaster.BT_AIEnemyMaster"))

(event `OnDie`)

(event `/Game/Blueprints/BPI_Enemy.ApplyDamageToEnemy`
  (params (Damage :type "Float (single-precision)"))
  (bind _health (`self.Health`))
  (if (> _health 0.0)
    (set `self.Health` (- _health Damage))
    (bind _asbp_fpshud (cast `/Game/Blueprints/Miscellaneous/BP_FPSHUD` (`PlayerController.GetHUD` (`GameplayStatics.GetPlayerController` 0))))
    (set `/Game/Blueprints/Miscellaneous/BP_FPSHUD.CanDrawHitCrosshair` true _asbp_fpshud)
    (`|ExecutionSequence`
      (:`then_0`
        (`self.SetHealthToWidget`)
        (`self.Die`))
      (:`then_1`
        (`KismetSystemLibrary.Delay` 0.2)
        (set `/Game/Blueprints/Miscellaneous/BP_FPSHUD.CanDrawHitCrosshair` false _asbp_fpshud)))))

(event `self.AIPerception.OnTargetPerceptionUpdated`
  (params (Actor :type "Actor Object Reference") (Stimulus :type "AIStimulus Structure"))
  (bind (_age _expirationage _strength _stimuluslocation _receiverlocation _tag _bsuccessfullysensed) (break `AIStimulus` Stimulus))
  (bind _returnvalue (`AIBlueprintHelperLibrary.GetBlackboard` self))
  (cast `/Game/Character/BP_FPSCharacter` Actor)
  (`BlackboardComponent.SetValueAsBool` _returnvalue "CanSeePlayerKey" _bsuccessfullysensed)
  (`BlackboardComponent.SetValueAsVector` _returnvalue "LastSeenLocation" _stimuluslocation))

(fn `UserConstructionScript`
  (`SceneComponent.K2_AttachToComponent` (`self.Gun`) (`self.Body`) "GripPoint" "SnapToTarget" "KeepRelative" "SnapToTarget" true))