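; Flying AI enemy running BT_AIFlier that grabs nearby physics objects and hurls them as damaging projectiles.
; Grab picks a random overlapping object, stores it in the blackboard, and uses a runtime physics handle, looping timer and timeline to hold it in front.
; Throw disables gravity, restores collision and applies a forward impulse; death also releases the object.
; A timeline-driven dash interpolates toward a flying point with random height offset.
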(event `self.ReceiveBeginPlay`
  (`parent.ReceiveBeginPlay`)
  (`self.SetBehaviorTree` "/Game/AIEnemies/AIFlier/BT_AIFlier.BT_AIFlier"))

(event `GrabObject`
  (bind _overlappingactors (`PrimitiveComponent.GetOverlappingActors` (`self.GrabCollision`) "/Game/Blueprints/BP_PhysicsObjectMaster.BP_PhysicsObjectMaster_C"))
  (bind _physicsobject (`/Game/Blueprints/BP_PhysicsObjectMaster.PhysicsObject` (`self.BP Physics Object`)))
  (bind _returnvalue (`KismetArrayLibrary.Array_Length` _overlappingactors))
  ;[0 1 0.6984] Grab Physics Object
  (if (!= _returnvalue 0)
    (bind _asbp_physics_object_master (cast `/Game/Blueprints/BP_PhysicsObjectMaster` (`|GetArrayItem` _overlappingactors (`KismetMathLibrary.RandomInteger` _returnvalue))))
    (bind _output_get (set `self.BP Physics Object` _asbp_physics_object_master))
    (`BlackboardComponent.SetValueAsObject` (`AIBlueprintHelperLibrary.GetBlackboard` self) "ObjectKey" _output_get)
    (bind _returnvalue_2 (`AddComponent|NODE_AddPhysicsHandleComponent-2` :`RelativeTransform` (`self.GetTransform`)))
    (set `self.Physics Handle` _returnvalue_2)
    (`PhysicsHandleComponent.GrabComponentAtLocation` (`self.Physics Handle`) _physicsobject "None" (`SceneComponent.K2_GetComponentLocation` _physicsobject))
    (`PrimitiveComponent.WakeRigidBody` _physicsobject "None")
    (`PrimitiveComponent.SetCollisionEnabled` _physicsobject "PhysicsOnly")
    (`PrimitiveComponent.SetCollisionResponseToChannel` _physicsobject "ECC_Pawn" "ECR_Ignore")
    (`PrimitiveComponent.SetCollisionResponseToChannel` _physicsobject "ECC_PhysicsBody" "ECR_Ignore")
    (`PrimitiveComponent.SetCollisionResponseToChannel` _physicsobject "ECC_Visibility" "ECR_Ignore")
    (set `self.Is Physics Handle Active` true)
    ;[0 0.5312 1] Set Physics Object Location
    (`KismetSystemLibrary.K2_SetTimerDelegate` (delegate `SetPhysicsObjectLocation`) 0.01 true)))

(event `SetPhysicsObjectLocation`
  (bind _capsulecomponent (`self.CapsuleComponent`))
  (bind _bp_physics_object (`self.BP Physics Object`))
  ;[0 0.5312 1] Set Physics Object Location
  (if (`self.Is Physics Handle Active`)
    (`/Engine/EditorBlueprintResources/StandardMacros.IsValid` (`self.Physics Handle`)
      (:`Is Valid`
        (`|ExecutionSequence`
          (:`then_0`
            (`/Engine/EditorBlueprintResources/StandardMacros.DoOnce` false :!label _label
              (:`Completed`
                (bind (_direction _alpha) (`Timeline|Move Object` :!via `PlayFromStart`)
                  (:`Update`
                    (`/Engine/EditorBlueprintResources/StandardMacros.IsValid` _bp_physics_object
                      (:`Is Valid`
                        _)))
                  (:`Finished`
                    (goto _label_2 :!via `Open`))))))
          (:`then_1`
            (`/Engine/EditorBlueprintResources/StandardMacros.Gate` true :!label _label_2
              (:`Exit`
                _))))
        (`PhysicsHandleComponent.SetTargetLocationAndRotation` (`self.Physics Handle`) (`KismetMathLibrary.VLerp` (`SceneComponent.K2_GetComponentLocation` (`/Game/Blueprints/BP_PhysicsObjectMaster.PhysicsObject` _bp_physics_object)) (+ (+ (`SceneComponent.K2_GetComponentLocation` _capsulecomponent) (* (`SceneComponent.GetForwardVector` _capsulecomponent) 150.0)) (0.0 0.0 20.0)) _alpha) (`self.K2_GetActorRotation`)))
      (:`Is Not Valid`
        (goto _label_2 :!via `Close`)))
    (else
      (goto _label :!via `Reset`))))

(event `ThrowObject`
  (bind _bp_physics_object (`self.BP Physics Object`))
  (bind _physicsobject (`/Game/Blueprints/BP_PhysicsObjectMaster.PhysicsObject` _bp_physics_object))
  ;[0.1928 0 1] Throw Physics Object
  (`/Engine/EditorBlueprintResources/StandardMacros.IsValid` _bp_physics_object
    (:`Is Valid`
      (`PhysicsHandleComponent.ReleaseComponent` (`self.Physics Handle`))
      (`PrimitiveComponent.SetEnableGravity` _physicsobject false)
      (`PrimitiveComponent.SetCollisionResponseToChannel` _physicsobject "ECC_Pawn" "ECR_Block")
      (`PrimitiveComponent.SetCollisionResponseToChannel` _physicsobject "ECC_PhysicsBody" "ECR_Block")
      (`PrimitiveComponent.SetCollisionResponseToChannel` _physicsobject "ECC_Visibility" "ECR_Block")
      (`PrimitiveComponent.SetCollisionEnabled` _physicsobject "QueryAndPhysics")
      (`PrimitiveComponent.AddImpulse` _physicsobject (* (`SceneComponent.GetForwardVector` (`self.CapsuleComponent`)) 8000.0) "None" true)
      (`|PlayMontage` (`self.Body`) "/Game/FPS_Assault_Pack/Animations/Rifle/A_Arms_Rifle_Shoot01_Montage.A_Arms_Rifle_Shoot01_Montage"
        (:`then`
          (`GameplayStatics.PlaySoundAtLocation` "/Game/Sounds/HitSounds/S_ThrowObject.S_ThrowObject" (`self.K2_GetActorLocation`) (struct) 1.0 1.0 0.0 null null null)
          (set `self.Is Physics Handle Active` false)
          (`BlackboardComponent.SetValueAsObject` (`AIBlueprintHelperLibrary.GetBlackboard` self) "ObjectKey" null)
          (`/Game/Blueprints/BP_PhysicsObjectMaster.ApplyDamageToPlayerEvent` (`self.BP Physics Object`)))))))

(event `self.OnDie`
  (bind _bp_physics_object (`self.BP Physics Object`))
  (bind _physics_handle (`self.Physics Handle`))
  (bind _physicsobject (`/Game/Blueprints/BP_PhysicsObjectMaster.PhysicsObject` _bp_physics_object))
  ;[1 0 0.0148] OnDie
  (`/Engine/EditorBlueprintResources/StandardMacros.IsValid` _physics_handle
    (:`Is Valid`
      (`PhysicsHandleComponent.ReleaseComponent` _physics_handle)
      (`/Engine/EditorBlueprintResources/StandardMacros.IsValid` _bp_physics_object
        (:`Is Valid`
          (`PrimitiveComponent.SetCollisionResponseToChannel` _physicsobject "ECC_Pawn" "ECR_Block")
          (`PrimitiveComponent.SetCollisionResponseToChannel` _physicsobject "ECC_PhysicsBody" "ECR_Block")
          (`PrimitiveComponent.SetCollisionResponseToChannel` _physicsobject "ECC_Visibility" "ECR_Block")
          (`PrimitiveComponent.SetCollisionEnabled` _physicsobject "QueryAndPhysics"))))))

(event `Dash`
  (params (FlyingPoint :type "Vector Structure"))
  ;[0 1 0.07784] Dash
  (set `self.TargetLocation` (`KismetMathLibrary.MakeVector` FlyingPoint_X FlyingPoint_Y (+ FlyingPoint_Z (`KismetMathLibrary.RandomFloatInRange` -300.0 300.0))))
  (bind (_direction _alpha) (`Timeline|DashMovement` :!via `PlayFromStart`)
    (:`Update`
      (`SceneComponent.K2_SetWorldLocation` (`self.CapsuleComponent`) (`KismetMathLibrary.VInterpTo` (`self.K2_GetActorLocation`) (`self.TargetLocation`) _alpha 1.0) true false))))

(fn `UserConstructionScript`
  (`parent.UserConstructionScript`))