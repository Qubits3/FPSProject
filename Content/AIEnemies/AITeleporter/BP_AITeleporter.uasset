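; BP_AITeleporter is an AI enemy that runs the BT_AITeleporter behavior tree and can dissolve and reappear.
; The construction script creates dynamic material instances for its body and gun.
; A shared Dissolve timeline drives the "Dissolve" parameter on both materials, played from the start by DissolveForward and reversed by DissolveReverse.
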(event `self.ReceiveBeginPlay`
  (`parent.ReceiveBeginPlay`)
  (`AIController.RunBehaviorTree` (`AIBlueprintHelperLibrary.GetAIController` self) "/Game/AIEnemies/AITeleporter/BT_AITeleporter.BT_AITeleporter"))

(event `DissolveForward`
  (bind (_direction _alpha) (`Timeline|Dissolve` :!via `PlayFromStart` :!label _label)
    (:`Update`
      (`MaterialInstanceDynamic.SetScalarParameterValue` (`self.BodyDynamicMaterial`) "Dissolve" _alpha)
      (`MaterialInstanceDynamic.SetScalarParameterValue` (`self.GunDynamicMaterial`) "Dissolve" _alpha))))

(event `DissolveReverse`
  (goto _label :!via `Reverse`))

(fn `UserConstructionScript`
  (`parent.UserConstructionScript`)
  (bind _returnvalue (`PrimitiveComponent.CreateDynamicMaterialInstance` (`self.Body`) 0 "/Game/AIEnemies/AITeleporter/Materials/MI_DissolveEffect.MI_DissolveEffect" "None"))
  (set `self.BodyDynamicMaterial` _returnvalue)
  (bind _returnvalue_2 (`PrimitiveComponent.CreateDynamicMaterialInstance` (`self.Gun`) 1 "/Game/FPS_Weapon_Bundle/Weapons/Materials/AR4/M_AR4.M_AR4" "None"))
  (set `self.GunDynamicMaterial` _returnvalue_2))