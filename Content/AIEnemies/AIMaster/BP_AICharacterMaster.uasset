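; Master AI enemy character for an FPS, providing health, locational damage, perception and death, with an empty OnDie event.
; Bone-name prefixes select damage multipliers, then hits update health and flash the HUD hit marker.
; BeginPlay starts the behavior tree and a timer toggling the health bar by trace distance, while sight and hearing feed the blackboard.
; Death awards score, ragdolls the body, hides the gun and destroys the actor later.
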(event `/Game/Blueprints/Interfaces/BPI_Enemy.ApplyDamageToEnemy`
  (params (Damage :type "Float (single-precision)") (BoneName :type String))
  ;[1 0 0] Multiply Damage Based on Body Parts
  (bind _properbonename (`self.ReturnProperBoneName` BoneName))
  (switch `string` _properbonename
    (:`Default`
      (`self.CalculateDamage` Damage))
    (:`head`
      (`GameplayStatics.PlaySoundAtLocation` "/Game/Sounds/HitSounds/S_HeadshotSound.S_HeadshotSound" (`self.K2_GetActorLocation`) (struct) 1.0 1.0 0.0 null null null)
      (`self.CalculateDamage` Damage 4.0))
    (:`pelvis`
      (`self.CalculateDamage` Damage 1.25 :!label _label))
    (:`spine`
      (goto _label))
    (:`clavicle`
      (goto _label))
    (:`thigh`
      (`self.CalculateDamage` Damage 0.75 :!label _label_2))
    (:`calf`
      (goto _label_2))
    (:`foot`
      (goto _label_2))
    (:`ball`
      (goto _label_2)))
  (`KismetSystemLibrary.Delay` 1.0))

(event `OnDie`
  ;[1 0.2469 0] Apply Damage
)

(event `ApplyCalculatedDamage`
  (bind _health (`self.Health`))
  ;[1 0.2469 0] Apply Damage
  (`AISense_Damage.ReportDamageEvent` self null 0.0 (`self.K2_GetActorLocation`))
  (if (> _health 0.0)
    (set `self.Health` (- _health (`self.MultipliedDamage`)))
    (bind _asbp_fpshud (cast `/Game/Blueprints/Miscellaneous/BP_FPSHUD` (`PlayerController.GetHUD` (`GameplayStatics.GetPlayerController` 0))))
    (set `/Game/Blueprints/Miscellaneous/BP_FPSHUD.CanDrawHitCrosshair` true _asbp_fpshud)
    (`|ExecutionSequence`
      (:`then_0`
        (`self.SetHealthToWidget`)
        (`self.Die`))
      (:`then_1`
        (`KismetSystemLibrary.Delay` 0.2)
        (set `/Game/Blueprints/Miscellaneous/BP_FPSHUD.CanDrawHitCrosshair` false _asbp_fpshud)))))

(event `SetWidgetVisibility`
  (params (NewVisibility :type Boolean))
  ;[0 1 0.00789] Set Health Widget Visibility Event
  (`SceneComponent.SetVisibility` (`self.HealthWidget`) NewVisibility false))

(event `SetVisibilityCallerEvent`
  ;[0 0.8597 1] Set Health Widget Visibility
  (`KismetSystemLibrary.K2_SetTimerDelegate` (delegate `SetVisibility`) 0.1 true))

(event `SetBehaviorTree`
  (params (BTAsset :type "BehaviorTree Object Reference"))
  ;[1 0 0] Every child class must call this event on BeginPlay
  (bind _asaicontroller (cast `AIController` (`self.GetController`)))
  (`AIController.RunBehaviorTree` _asaicontroller BTAsset))

(event `SetVisibility`
  ;[0 0.8597 1] Set Health Widget Visibility
  (if (`self.WasRecentlyRendered` 0.1)
    (bind _asbp_fpscharacter (cast `/Game/Character/BP_FPSCharacter` (`GameplayStatics.GetPlayerCharacter` 0)))
    (bind _outhit (`KismetSystemLibrary.LineTraceSingle` (`self.K2_GetActorLocation`) (`self.K2_GetActorLocation` _asbp_fpscharacter) "TraceTypeQuery4"))
    (if (< (`.Distance` (`GameplayStatics.BreakHitResult` _outhit)) 1000.0)
      (`self.SetWidgetVisibility` true)
      (else
        (`self.SetWidgetVisibility` false)))))

(event `self.ReceiveBeginPlay`
  (`self.SetHealthToWidget`)
  (`self.SetBehaviorTree` "/Game/AIEnemies/AIMaster/BT_AIEnemyMaster.BT_AIEnemyMaster")
  (`self.SetVisibilityCallerEvent`))

(event `self.AIPerception.OnPerceptionUpdated`
  (params (UpdatedActors :type "Array of Actor Object Reference (by ref)"))
  (bind _returnvalue (`AIBlueprintHelperLibrary.GetBlackboard` self))
  ;[1 0.9987 0] AI Perception
  (for _array_element UpdatedActors
    (bind _info (`AIPerceptionComponent.GetActorsPerception` (`self.AIPerception`) _array_element))
    (for _array_element_2 (`.LastSensedStimuli` (break `ActorPerceptionBlueprintInfo` _info))
      (bind _returnvalue_2 (`AIPerceptionSystem.GetSenseClassForStimulus` _array_element_2))
      (switch `string` (`KismetSystemLibrary.GetClassDisplayName` _returnvalue_2)
        (:`AISense_Sight`
          (bind (_age _expirationage _strength _stimuluslocation _receiverlocation _tag _bsuccessfullysensed) (break `AIStimulus` _array_element_2))
          (`BlackboardComponent.SetValueAsBool` _returnvalue "CanSeePlayerKey" _bsuccessfullysensed))
        (:`AISense_Hearing`
          (`BlackboardComponent.SetValueAsBool` _returnvalue "CanHearPlayerKey" _bsuccessfullysensed)
          (`BlackboardComponent.SetValueAsVector` _returnvalue "LastSeenLocation" _stimuluslocation)
          (`KismetSystemLibrary.Delay` 0.5)
          (`BlackboardComponent.SetValueAsBool` _returnvalue "CanHearPlayerKey" false))))))

(event `FaceToCharacterSmoothlyByTag`
  (params (AIEnemy :type "/Game/AIEnemies/AIMaster/BP_AICharacterMaster Object Reference"))
  (cast `/Game/Character/BP_FPSCharacter` (`BlackboardComponent.GetValueAsObject` (`AIBlueprintHelperLibrary.GetBlackboard` self) "PlayerKey"))
  (bind (_direction _alpha) (`Timeline|RotateSmoothly` :!via `PlayFromStart`)))

(fn `UserConstructionScript`
  (`SceneComponent.K2_AttachToComponent` (`self.Gun`) (`self.Body`) "GripPoint" "SnapToTarget" "KeepRelative" "SnapToTarget" true))