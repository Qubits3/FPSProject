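; BP_AITurret is an AI turret enemy that starts the BT_AITurret behavior tree on BeginPlay.
; Its RotateSlowly event runs a timeline that eases the AI controller's control rotation toward the player's BP_FPSCharacter, feeding the timeline alpha into RInterpTo as delta time.
; When the timeline finishes, the controller sets focus on the player so the turret keeps facing them.
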(event `self.ReceiveBeginPlay`
  (`parent.ReceiveBeginPlay`)
  (`self.SetBehaviorTree` "/Game/AIEnemies/AITurret/BT_AITurret.BT_AITurret"))

(event `self.ReceiveTick`
  (params (DeltaSeconds :type "Float (single-precision)")))

(event `RotateSlowly`
  (bind _asbp_fpscharacter (cast `/Game/Character/BP_FPSCharacter` (`Controller.K2_GetPawn` (`GameplayStatics.GetPlayerController` 0))))
  (bind (_direction _alpha) (`Timeline|RotateTurret` :!via `PlayFromStart`)
    (:`Update`
      (`Controller.SetControlRotation` (`AIBlueprintHelperLibrary.GetAIController` self) (`KismetMathLibrary.RInterpTo` (`self.K2_GetActorRotation`) (`KismetMathLibrary.FindLookAtRotation` (`self.K2_GetActorLocation`) (`self.K2_GetActorLocation` _asbp_fpscharacter)) _alpha 1.0)))
    (:`Finished`
      (`AIController.K2_SetFocus` (`AIBlueprintHelperLibrary.GetAIController` self) _asbp_fpscharacter))))

(fn `UserConstructionScript`
  (`parent.UserConstructionScript`))