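; BP_AICharacterMaster is an AI enemy character with a gun attached to its body, a health bar widget and a behavior tree.
; Perception updates write whether the BP_FPSCharacter is seen, and its last stimulus location, to the blackboard.
; Each projectile hit subtracts fixed health and refreshes the bar.
; At exactly zero health it flags death in the blackboard, ragdolls, hides the gun and bar, then destroys itself after a delay.
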(event `self.ReceiveBeginPlay`
  (`self.SetHealthToWidget`)
  (`AIController.RunBehaviorTree` (`AIBlueprintHelperLibrary.GetAIController` self) "/Game/AIEnemy/BT_AIEnemy.BT_AIEnemy"))

(event `/Game/Blueprints/BPI_Damage.ApplyProjectileDamageToEnemy`
  (bind _health (`self.Health`))
  (if (> _health 0.0)
    (set `self.Health` (- _health 10.0))
    (`self.SetHealthToWidget`)
    (`self.Die`)))

(event `self.AIPerception.OnTargetPerceptionUpdated`
  (params (Actor :type "Actor Object Reference") (Stimulus :type "AIStimulus Structure"))
  (bind (_age _expirationage _strength _stimuluslocation _receiverlocation _tag _bsuccessfullysensed) (break `AIStimulus` Stimulus))
  (bind _returnvalue (`AIBlueprintHelperLibrary.GetBlackboard` null))
  (cast `/Game/Character/BP_FPSCharacter` Actor)
  (`BlackboardComponent.SetValueAsBool` _returnvalue "CanSeePlayerKey" _bsuccessfullysensed)
  (`BlackboardComponent.SetValueAsVector` _returnvalue "LastSeenLocation" _stimuluslocation))

(fn `UserConstructionScript`
  (`SceneComponent.K2_AttachToComponent` (`self.Gun`) (`self.Body`) "GripPoint" "SnapToTarget" "KeepRelative" "SnapToTarget" true))