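; BP_LevelStreamer is a trigger actor that streams levels when the player walks into its box.
; When enabled, an overlap by the player's BP_FPSCharacter loads the chosen level visible, optionally blocking, and can also unload another level.
; Levels are picked through enum values converted to names.
; The construction script changes the editor billboard sprite and scale to show whether the streamer is enabled.
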(event `self.Box.OnComponentBeginOverlap`
  (params (OverlappedComponent :type "PrimitiveComponent Object Reference") (OtherActor :type "Actor Object Reference") (OtherComp :type "PrimitiveComponent Object Reference") (OtherBodyIndex :type Integer) (bFromSweep :type Boolean) (SweepResult :type "HitResult Structure (by ref)"))
  (bind _asbp_fpscharacter (cast `/Game/Character/BP_FPSCharacter` (`GameplayStatics.GetPlayerCharacter` 0)))
  (if (`self.isEnabled`)
    (if (== OtherActor _asbp_fpscharacter)
      (`GameplayStatics.LoadStreamLevel` (`KismetStringLibrary.Conv_StringToName` (`|GetEnumeratorNameAsString` (`self.LoadLevel`))) true (`self.BlockOnLoad`))
      (if (`self.ShouldUnloadLevel`)
        (`GameplayStatics.UnloadStreamLevel` (`KismetStringLibrary.Conv_StringToName` (`|GetEnumeratorNameAsString` (`self.UnloadLevel`))))))))

(fn `UserConstructionScript`
  (bind _billboard (`self.Billboard`))
  (if (`self.isEnabled`)
    (`BillboardComponent.SetSprite` _billboard "/Engine/EditorResources/S_Actor.S_Actor")
    (set `self.SpriteScale` 2.0)
    (else
      (`BillboardComponent.SetSprite` _billboard "/Game/Textures/T_Cross.T_Cross")
      (set `self.SpriteScale` 0.5))))