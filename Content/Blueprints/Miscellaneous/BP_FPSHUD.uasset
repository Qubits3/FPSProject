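; HUD Blueprint that draws a procedural first-person crosshair at the centre of the screen.
; DrawHUD uses DrawLine to render four arms around a gap, driven by length, spacing, colour and thickness variables.
; When CanDrawHitCrosshair is true it adds four thin diagonal strokes as a hit marker; this graph only reads that flag.
; A centre dot is present but unconnected, so it never draws.
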(event `self.ReceiveDrawHUD`
  (params (SizeX :type Integer) (SizeY :type Integer))
  (bind _halfx (`self.HalfX`))
  (bind _halfy (`self.HalfY`))
  (bind _halfy_2 (`self.HalfY`))
  (bind _halfx_2 (`self.HalfX`))
  (bind _halfy_3 (`self.HalfY`))
  (bind _halfx_3 (`self.HalfX`))
  (bind _halfy_4 (`self.HalfY`))
  (bind _halfx_4 (`self.HalfX`))
  (bind _halfy_5 (`self.HalfY`))
  (bind _halfx_5 (`self.HalfX`))
  (bind _halfy_6 (`self.HalfY`))
  (bind _crosshair_space (`self.Crosshair Space`))
  (bind _crosshair_space_2 (`self.Crosshair Space`))
  (bind _crosshair_space_3 (`self.Crosshair Space`))
  (bind _crosshair_space_4 (`self.Crosshair Space`))
  (bind _halfx_6 (`self.HalfX`))
  (bind _halfy_7 (`self.HalfY`))
  (bind _halfx_7 (`self.HalfX`))
  (bind _halfy_8 (`self.HalfY`))
  (bind _halfx_8 (`self.HalfX`))
  (bind _returnvalue (- (`self.Crosshair Length`) 3.0))
  (bind _returnvalue_2 (- (`self.Crosshair Length`) 3.0))
  (bind _returnvalue_3 (- (`self.Crosshair Length`) 3.0))
  (bind _returnvalue_4 (- (`self.Crosshair Length`) 3.0))
  (set `self.HalfX` (`KismetMathLibrary.Conv_IntToDouble` (/ SizeX 2)))
  (set `self.HalfY` (`KismetMathLibrary.Conv_IntToDouble` (/ SizeY 2)))
  ;[1 1 1] Horizontal Lines
  (`self.DrawLine` (+ _halfx_6 (`self.Crosshair Length`)) _halfy_7 (+ _halfx_6 (`self.Crosshair Space`)) _halfy_7 (`self.Crosshair Color`) (`self.Crosshair Thickness`))
  (`self.DrawLine` (- _halfx_7 (`self.Crosshair Length`)) _halfy_8 (- _halfx_7 (`self.Crosshair Space`)) _halfy_8 (`self.Crosshair Color`) (`self.Crosshair Thickness`))
  ;[1 1 1] Vertical Lines
  (`self.DrawLine` _halfx_8 (+ _halfy_2 (`self.Crosshair Length`)) _halfx_8 (+ _halfy_2 (`self.Crosshair Space`)) (`self.Crosshair Color`) (`self.Crosshair Thickness`))
  (`self.DrawLine` _halfx (- _halfy (`self.Crosshair Length`)) _halfx (- _halfy (`self.Crosshair Space`)) (`self.Crosshair Color`) (`self.Crosshair Thickness`))
  ;[1 1 1] Hit Crosshair
  (if (`self.CanDrawHitCrosshair`)
    (`self.DrawLine` (- _halfx_4 _crosshair_space_2) (- _halfy_3 _crosshair_space_2) (- _halfx_4 _returnvalue_2) (- _halfy_3 _returnvalue_2) (`self.Crosshair Color`) 1.0)
    (`self.DrawLine` (+ _halfx_3 _crosshair_space_3) (- _halfy_5 _crosshair_space_3) (+ _halfx_3 _returnvalue_3) (- _halfy_5 _returnvalue_3) (`self.Crosshair Color`) 1.0)
    (`self.DrawLine` (- _halfx_5 _crosshair_space_4) (+ _halfy_6 _crosshair_space_4) (- _halfx_5 _returnvalue_4) (+ _halfy_6 _returnvalue_4) (`self.Crosshair Color`) 1.0)
    (`self.DrawLine` (+ _halfx_2 _crosshair_space) (+ _halfy_4 _crosshair_space) (+ _halfx_2 _returnvalue) (+ _halfy_4 _returnvalue) (`self.Crosshair Color`) 1.0)))

(fn `UserConstructionScript`)