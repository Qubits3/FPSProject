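; Spawner actor that places randomly chosen classes from an Objects array at half scale and tracks them for later removal.
; SpawnObjects makes ObjectCount attempts, adjusting for collisions or skipping blocked spawns, and DeleteObjects destroys and clears the tracked actors.
; Each location comes from CalculateSpawnLocation, whose visible random Box-bounds math, inset and offset by actor location, is left unused.
; The construction script only holds a disconnected debug print of scaled box extent.
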(event `SpawnObjects`
  (bind _objects (`self.Objects`))
  (for _ (range (+ (`self.ObjectCount`) 1))
    (bind _returnvalue (`|SpawnActorFromClass` (`|GetArrayItem` _objects (`KismetMathLibrary.RandomInteger` (`KismetArrayLibrary.Array_Length` _objects))) (`KismetMathLibrary.MakeTransform` (`self.CalculateSpawnLocation`) (struct) (0.5 0.5 0.5)) "AdjustIfPossibleButDontSpawnIfColliding" "OverrideRootScale" null null))
    (`KismetArrayLibrary.Array_Add` (`self.SpawnedObjects`) _returnvalue)))

(event `DeleteObjects`
  (bind _spawnedobjects (`self.SpawnedObjects`))
  (for _array_element _spawnedobjects
    (`self.K2_DestroyActor` _array_element))
  (`KismetArrayLibrary.Array_Clear` _spawnedobjects))

(fn `UserConstructionScript`)