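; BP_ArenaDoor is a sliding arena door that opens when a BP_FPSCharacter enters its trigger box and closes when one leaves.
; Overlap events on Collider call OpenDoor and CloseDoor, which play a sound and use eased MoveComponentTo to raise Door or return it to zero relative location.
; The construction script enlarges the Arrow, sizes Collider from BoxExtent and offsets it along X to match that extent.
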(event `self.Collider.OnComponentBeginOverlap`
  (params (OverlappedComponent :type "PrimitiveComponent Object Reference") (OtherActor :type "Actor Object Reference") (OtherComp :type "PrimitiveComponent Object Reference") (OtherBodyIndex :type Integer) (bFromSweep :type Boolean) (SweepResult :type "HitResult Structure (by ref)"))
  (cast `/Game/Character/BP_FPSCharacter` OtherActor)
  (`self.OpenDoor`))

(event `self.Collider.OnComponentEndOverlap`
  (params (OverlappedComponent :type "PrimitiveComponent Object Reference") (OtherActor :type "Actor Object Reference") (OtherComp :type "PrimitiveComponent Object Reference") (OtherBodyIndex :type Integer))
  (cast `/Game/Character/BP_FPSCharacter` OtherActor)
  (`self.CloseDoor`))

(event `OpenDoor`
  (`GameplayStatics.PlaySoundAtLocation` "/Game/Sounds/S_SlidingDoorOpen.S_SlidingDoorOpen" (`self.K2_GetActorLocation`) (struct) 1.0 1.0 0.0 null null null)
  (`KismetSystemLibrary.MoveComponentTo` (`self.Door`) (0.0 0.0 100.0) (struct) true true 3.51))

(event `CloseDoor`
  (`GameplayStatics.PlaySoundAtLocation` "/Game/Sounds/S_SlidingDoorClose.S_SlidingDoorClose" (`self.K2_GetActorLocation`) (struct) 1.0 1.0 0.0 null null null)
  (`KismetSystemLibrary.MoveComponentTo` (`self.Door`) (0.0 0.0 0.0) (struct) true true 3.69))

(fn `UserConstructionScript`
  (bind _collider (`self.Collider`))
  (bind _boxextent (`self.BoxExtent`))
  (`SceneComponent.SetWorldScale3D` (`self.Arrow`) (5.0 5.0 5.0))
  (`BoxComponent.SetBoxExtent` _collider (`KismetMathLibrary.MakeVector` _boxextent 50.0 50.0) true)
  (`SceneComponent.K2_AddRelativeLocation` _collider (`KismetMathLibrary.MakeVector` (+ _boxextent 50.0)) false true))