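; BP_Launcher is a launch pad that flings the FPS character when it overlaps the box.
; The overlap handler sums the character root's up and forward vectors, each scaled by LaunchPower, and passes the result to LaunchCharacter, overriding existing XY and Z velocity.
; Launch direction therefore follows the character's facing rather than the pad's orientation.
; A disconnected debug branch prints a camera-based version of the same vector and never runs.
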(event `self.ReceiveTick`
  (params (DeltaSeconds :type "Float (single-precision)"))
  ;[1 1 1] Debug
)

(event `self.Box.OnComponentBeginOverlap`
  (params (OverlappedComponent :type "PrimitiveComponent Object Reference") (OtherActor :type "Actor Object Reference") (OtherComp :type "PrimitiveComponent Object Reference") (OtherBodyIndex :type Integer) (bFromSweep :type Boolean) (SweepResult :type "HitResult Structure (by ref)"))
  (bind _launch_power (`self.Launch Power`))
  (bind _asbp_fpscharacter (cast `/Game/Blueprints/BP_FPSCharacter` OtherActor))
  (bind _rootcomponent (`Actor.RootComponent` _asbp_fpscharacter))
  (`Character.LaunchCharacter` _asbp_fpscharacter (+ (* (`SceneComponent.GetUpVector` _rootcomponent) _launch_power) (* (`SceneComponent.GetForwardVector` _rootcomponent) _launch_power)) true true))

(fn `UserConstructionScript`)