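; Enemy spawner actor that, when enabled, spawns random AI pawns on a one-second looping timer.
; Each tick increments EnemyCount, even past MaxEnemyCount; under the cap it async-loads a class and an independently randomised Behavior Tree before spawning.
; AddScore decrements the count on enemy death, and the construction script swaps the billboard sprite by enabled state.
; CalculateSpawnLocation's random point-in-Box calculation is left unconnected.
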(event `Print`
  ;[1 1 1] Debug
  (`KismetSystemLibrary.PrintString` (`KismetStringLibrary.Conv_VectorToString` (`.BoxExtent` (`KismetSystemLibrary.GetComponentBounds` (`self.Box`)))) true true (struct :`R` 1.0 :`G` 1.0 :`B` 1.0 :`A` 1.0) 10.0))

(event `self.ReceiveBeginPlay`
  (if (`self.IsEnabled`)
    (`KismetSystemLibrary.K2_SetTimerDelegate` (delegate `SpawnEnemy`) 1.0 true)))

(event `SpawnEnemy`
  (bind _aienemyclass (`self.AIEnemyClass`))
  (bind _returnvalue (`KismetMathLibrary.RandomInteger` (`KismetArrayLibrary.Array_Length` _aienemyclass)))
  (`/Engine/EditorBlueprintResources/StandardMacros.IncrementFloat` (`self.EnemyCount`)
    (:`  `
      (if (<= (`self.EnemyCount`) (`self.MaxEnemyCount`))
        (bind _class (`|LoadAssetClass` (`|GetArrayItem` _aienemyclass _returnvalue))
          (:`Completed`
            (bind _aspawn (castclass `Pawn` _class))
            (bind _object (`|LoadAsset` (`|GetArrayItem` (`self.Behavior Tree`) _returnvalue))
              (:`Completed`
                (bind _asbehavior_tree (cast `BehaviorTree` _object))
                (`AIBlueprintHelperLibrary.SpawnAIFromClass` _aspawn _asbehavior_tree (`self.CalculateSpawnLocation`) (struct) false null)))))))))

(event `/Game/Blueprints/BPI_CharacterInfo.AddScore`
  (params (ScorePoint :type "Float (single-precision)"))
  ;[1 1 1] Enemy is dead
  (`/Engine/EditorBlueprintResources/StandardMacros.DecrementFloat` (`self.EnemyCount`)))

(fn `UserConstructionScript`
  (bind _billboard (`self.Billboard`))
  (if (`self.IsEnabled`)
    (`BillboardComponent.SetSprite` _billboard "/Engine/EditorResources/Ai_Spawnpoint.Ai_Spawnpoint")
    (set `self.SpriteScale` 5.0)
    (else
      (`BillboardComponent.SetSprite` _billboard "/Engine/EngineResources/AICON-Red.AICON-Red")
      (set `self.SpriteScale` 10.0))))