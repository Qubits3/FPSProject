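; BP_GrappleHook is the grapple hook projectile that pulls the first-person player character when it hits something.
; On BeginPlay it sets its ProjectileMovement velocity from the gun's Muzzle socket toward the character's last line-trace hit, scaling the unnormalized offset so speed grows with distance.
; Any hit on its Collision component calls PullCharacterEvent on player 0's BP_FPSCharacter, which handles the pull.
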(event `self.ReceiveBeginPlay`
  (bind _asbp_fpscharacter (cast `/Game/Blueprints/BP_FPSCharacter` (`GameplayStatics.GetPlayerCharacter` 0)))
  (set `MovementComponent.Velocity` (* (- (`/Game/Blueprints/BP_FPSCharacter.LineLastHitLocation` _asbp_fpscharacter) (`SceneComponent.GetSocketLocation` (`/Game/Blueprints/BP_FPSCharacter.Gun` _asbp_fpscharacter) "Muzzle")) 1500.0) (`self.ProjectileMovement`)))

(event `self.Collision.OnComponentHit`
  (params (HitComponent :type "PrimitiveComponent Object Reference") (OtherActor :type "Actor Object Reference") (OtherComp :type "PrimitiveComponent Object Reference") (NormalImpulse :type "Vector Structure") (Hit :type "HitResult Structure (by ref)"))
  (bind _asbp_fpscharacter (cast `/Game/Blueprints/BP_FPSCharacter` (`GameplayStatics.GetPlayerCharacter` 0)))
  (`/Game/Blueprints/BP_FPSCharacter.PullCharacterEvent` _asbp_fpscharacter))

(fn `UserConstructionScript`)