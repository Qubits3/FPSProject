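; BP_Ladder is a ladder actor that procedurally builds its metal steps in the construction script.
; It derives the step count and starting height from the StaticMesh bounds and StepSpacing, offset from the Obstacle component.
; A loop adds scaled cube mesh components upward at even world-space intervals, after running the parent construction script.
; The event graph has no active logic.
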(fn `UserConstructionScript`
  (bind (_returnvalue_x _returnvalue_y _returnvalue_z) (`KismetMathLibrary.BreakVector` (`SceneComponent.K2_GetComponentScale` (`self.Obstacle`))))
  (bind (_origin _boxextent) (`KismetSystemLibrary.GetComponentBounds` (`self.StaticMesh`)))
  (`parent.UserConstructionScript`)
  (`|ExecutionSequence`
    (:`then_0`
      ;[1 1 1] Setup variables
      (set `self.Box Extent Z` (.z _boxextent))
      (set `self.StairStepCount` (* (/ (.z _boxextent) (`self.StepSpacing`)) 2.0))
      (set `self.NewStepLocation` (`KismetMathLibrary.MakeVector` 0.0 0.0 (* (+ (.z _boxextent) (+ _returnvalue_z (/ (`self.StepSpacing`) 2.0))) -1.0))))
    (:`then_1`
      ;[1 1 1] Add Stair Steps
      (for _ (range 1 (+ (`KismetMathLibrary.FTrunc` (`self.StairStepCount`)) 1))
        (bind _returnvalue (`AddComponent|NODE_AddStaticMeshComponent-2`))
        (`StaticMeshComponent.SetStaticMesh` _returnvalue "/Engine/BasicShapes/Cube.Cube")
        (`PrimitiveComponent.SetMaterial` _returnvalue 0 "/Game/Materials/MI_Metal.MI_Metal")
        (`SceneComponent.SetWorldScale3D` _returnvalue (0.08 0.6 0.05))
        (bind _output_get (set `self.NewStepLocation` (+ (`self.NewStepLocation`) (`KismetMathLibrary.MakeVector` 0.0 0.0 (`self.StepSpacing`)))))
        (`SceneComponent.K2_SetWorldLocation` _returnvalue (+ _output_get (`SceneComponent.K2_GetComponentLocation` (`self.Obstacle`))) false false)))))