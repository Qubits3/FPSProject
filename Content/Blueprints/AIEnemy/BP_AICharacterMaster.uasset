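; Master Blueprint for AI enemy characters, handling health, projectile damage and death.
; Each projectile hit removes a fixed amount of health, updates the WP_HealthBar in the HealthWidget component and runs the death check.
; At exactly zero health, the mesh ragdolls, capsule collision turns off, the health widget is cleared and the actor is destroyed after a delay.
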(event `self.ReceiveBeginPlay`
  (`self.SetHealthToWidget`))

(event `/Game/Blueprints/BPI_Damage.ApplyProjectileDamage`
  (bind _health (`self.Health`))
  (if (> _health 0.0)
    (set `self.Health` (- _health 10.0))
    (`self.SetHealthToWidget`)
    (`self.Die`)))

(fn `UserConstructionScript`)