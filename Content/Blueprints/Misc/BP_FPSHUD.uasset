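; BP_FPSHUD is a first-person HUD that draws a simple four-line crosshair at the screen center.
; On each DrawHUD event it halves the viewport size to find the center, then draws horizontal and vertical line pairs with a gap in the middle.
; Variables control the crosshair's length, center spacing, color and thickness.
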(event `self.ReceiveDrawHUD`
  (params (SizeX :type Integer) (SizeY :type Integer))
  (bind _halfx (`self.HalfX`))
  (bind _halfy (`self.HalfY`))
  (bind _halfy_2 (`self.HalfY`))
  (bind _halfx_2 (`self.HalfX`))
  (bind _halfy_3 (`self.HalfY`))
  (bind _halfx_3 (`self.HalfX`))
  (bind _halfy_4 (`self.HalfY`))
  (bind _halfx_4 (`self.HalfX`))
  (set `self.HalfX` (`KismetMathLibrary.Conv_IntToDouble` (/ SizeX 2)))
  (set `self.HalfY` (`KismetMathLibrary.Conv_IntToDouble` (/ SizeY 2)))
  ;[1 1 1] Horizontal Lines
  (`self.DrawLine` (+ _halfx_2 (`self.Crosshair Length`)) _halfy_3 (+ _halfx_2 (`self.Crosshair Space`)) _halfy_3 (`self.Crosshair Color`) (`self.Crosshair Thickness`))
  (`self.DrawLine` (- _halfx_3 (`self.Crosshair Length`)) _halfy_4 (- _halfx_3 (`self.Crosshair Space`)) _halfy_4 (`self.Crosshair Color`) (`self.Crosshair Thickness`))
  ;[1 1 1] Vertical Lines
  (`self.DrawLine` _halfx_4 (+ _halfy_2 (`self.Crosshair Length`)) _halfx_4 (+ _halfy_2 (`self.Crosshair Space`)) (`self.Crosshair Color`) (`self.Crosshair Thickness`))
  (`self.DrawLine` _halfx (- _halfy (`self.Crosshair Length`)) _halfx (- _halfy (`self.Crosshair Space`)) (`self.Crosshair Color`) (`self.Crosshair Thickness`)))

(fn `UserConstructionScript`)