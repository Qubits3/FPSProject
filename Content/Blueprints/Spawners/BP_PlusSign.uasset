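; BP_PlusSign is a health pickup whose plus sign rotates and moves via RotatingMovement and InterpToMovement components.
; Any actor overlapping the Sphere is sent an AddPlayerHealth message with a fixed amount.
; The sign then hides and CanHeal clears for a short delay before both restore.
; CanHeal is never checked here, so overlaps during the delay still send healing.
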(event `self.Sphere.OnComponentBeginOverlap`
  (params (OverlappedComponent :type "PrimitiveComponent Object Reference") (OtherActor :type "Actor Object Reference") (OtherComp :type "PrimitiveComponent Object Reference") (OtherBodyIndex :type Integer) (bFromSweep :type Boolean) (SweepResult :type "HitResult Structure (by ref)"))
  (message `/Game/Blueprints/Interfaces/BPI_Player.AddPlayerHealth` OtherActor 50.0)
  (`SceneComponent.SetVisibility` (`self.PlusSign`) false false)
  (set `self.CanHeal` false)
  (`KismetSystemLibrary.Delay` 2.0)
  (`SceneComponent.SetVisibility` (`self.PlusSign`) true false)
  (set `self.CanHeal` true))

(event `self.ReceiveBeginPlay`
  (`MovementComponent.SetUpdatedComponent` (`self.RotatingMovement`) (`self.PlusSign`))
  (`MovementComponent.SetUpdatedComponent` (`self.InterpToMovement`) (`self.PlusSign`)))

(fn `UserConstructionScript`)