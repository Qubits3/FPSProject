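; BP_ObjectSpawner is a spawner actor that scatters random objects from a class list, sized and placed relative to its Box component.
; SpawnObjects creates up to ObjectCount actors at CalculateSpawnLocation with random per-axis scale, skipping colliding placements.
; Each actor shifts down by the difference between box and actor half-heights, then joins SpawnedObjects for DeleteObjects to clear.
; A Print event displays the box extent for debugging.
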(event `Print`
  (`KismetSystemLibrary.PrintString` (`KismetStringLibrary.Conv_VectorToString` (`.BoxExtent` (`KismetSystemLibrary.GetComponentBounds` (`self.Box`)))) true true (struct :`R` 1.0 :`G` 1.0 :`B` 1.0 :`A` 1.0) 10.0))

(event `SpawnObjects`
  (bind _returnvalue (`KismetMathLibrary.RandomFloatInRange` 0.3 0.5))
  (bind _objects (`self.Objects`))
  (for _ (range 1 (+ (`self.ObjectCount`) 1))
    (bind _returnvalue_2 (`|SpawnActorFromClass` (`|GetArrayItem` _objects (`KismetMathLibrary.RandomInteger` (`KismetArrayLibrary.Array_Length` _objects))) (`KismetMathLibrary.MakeTransform` (`self.CalculateSpawnLocation`) (struct) (`KismetMathLibrary.MakeVector` _returnvalue _returnvalue _returnvalue)) "DontSpawnIfColliding" "OverrideRootScale" null null))
    (`self.K2_AddActorWorldOffset` _returnvalue_2 (`KismetMathLibrary.MakeVector` 0.0 0.0 (* (- (.z (`.BoxExtent` (`KismetSystemLibrary.GetComponentBounds` (`self.Box`)))) (.z (`.BoxExtent` (`self.GetActorBounds` _returnvalue_2 false false)))) -1.0)) false false)
    (`KismetArrayLibrary.Array_Add` (`self.SpawnedObjects`) _returnvalue_2)))

(event `DeleteObjects`
  (bind _spawnedobjects (`self.SpawnedObjects`))
  (for _array_element _spawnedobjects
    (`self.K2_DestroyActor` _array_element))
  (`KismetArrayLibrary.Array_Clear` _spawnedobjects))

(fn `UserConstructionScript`)