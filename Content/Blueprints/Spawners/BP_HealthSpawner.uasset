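; BP_HealthSpawner is a health spawner actor marked by a plus-sign component, with no spawning logic in these graphs.
; When AutoLocate is set, its construction script traces the Visibility channel down the plus sign's local axis to find a surface.
; It then moves the actor slightly below the hit point, without checking that the trace hit anything.
; The event graph holds only disabled placeholder events.
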(fn `UserConstructionScript`
  (bind _bp_plussign (`self.BP_PlusSign`))
  (bind _returnvalue (`SceneComponent.K2_GetComponentLocation` _bp_plussign))
  (if (`self.AutoLocate`)
    (bind _outhit (`KismetSystemLibrary.LineTraceSingle` _returnvalue (+ _returnvalue (* (* (`SceneComponent.GetUpVector` _bp_plussign) -1.0) 2000.0)) "TraceTypeQuery1"))
    (`self.K2_SetActorLocation` (- (`.Location` (`GameplayStatics.BreakHitResult` _outhit)) (0.0 0.0 40.0)))))